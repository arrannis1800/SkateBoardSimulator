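; BP_StaticFunctions is a set of shared helper functions for reaching the game's core objects.
; GetGM returns the current game mode cast to BP_ThirdPersonGameMode, and GetMainHUD builds on it to return that game mode's HUD reference.
; GetPlayer returns player 0's character cast to BP_ThirdPersonCharacter.
; Both casts have no fallback, so execution simply stops when the type does not match.
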(fn GetGM
  (bind _asbp_third_person_game_mode (Utilities|Casting|CastToBP_ThirdPersonGameMode (Game|GetGameMode)))
  (return _asbp_third_person_game_mode))

(fn GetMainHUD
  (return (Variables|/Game/Blueprints/BP_ThirdPersonGameMode.BP_ThirdPersonGameMode_C|GetHUD (CallFunction|GetGM))))

(fn GetPlayer
  (bind _asbp_third_person_character (Utilities|Casting|CastToBP_ThirdPersonCharacter (Game|GetPlayerCharacter 0)))
  (return _asbp_third_person_character))